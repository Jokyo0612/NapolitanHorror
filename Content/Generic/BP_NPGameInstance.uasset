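; BP_NPGameInstance is a Game Instance Blueprint that handles the game-over sequence.
; On Init it binds to OnGameStateChanged and reacts only to the Game Over state.
; That state fades out the player camera and holds it, then after a matching delay hides the player controller's default UI.
; It then async-loads the WBP_LooseScreen widget class, creates it and adds it to the viewport.
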(event `self.ReceiveInit`
  (add `self.OnGameStateChanged` (delegate `OnGameStateChanged_이벤트`)))

(event `OnGameStateChanged_이벤트` :!signature `self.OnGameStateChanged`
  (params (CurrentState :type "ENPGameState Enum" :default "WaitingToStart"))
  (switch `ENPGameState` CurrentState
    (:`GameOver`
      ; Dead Logic
      (`PlayerCameraManager.StartCameraFade` :`self` (`GameplayStatics.GetPlayerCameraManager` 0) :`ToAlpha` 1.0 :`Duration` 2.0 :`bHoldWhenFinished` true)
      (`KismetSystemLibrary.Delay` 2.0)
      (bind _asnpplayer_controller (cast `NPPlayerController` (`GameplayStatics.GetPlayerController` 0)))
      (`Widget.SetVisibility` (`NPPlayerController.DefaultUI` _asnpplayer_controller) "Hidden")
      (bind _class (`|LoadAssetClass` "/Game/Widget/Menu/WBP_LooseScreen.WBP_LooseScreen_C")
        (:`Completed`
          (bind `_as사용자_위젯` (castclass `UserWidget` _class))
          (bind _returnvalue (`|CreateWidget` `_as사용자_위젯`))
          (`UserWidget.AddToViewport` _returnvalue 0))))))