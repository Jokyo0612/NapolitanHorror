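; Tutorial game mode Blueprint that shows the tutorial widget and scripts the narration sequence leading to the end of the tutorial chapter.
; When the owning player's narration component initializes, it listens for the Call.00.Tutorial narration to end, then triggers Sub.00.Room2 after a short delay.
; When that narration ends, it waits again and calls EndChapter with Chapter.00.Warehouse.
; Each one-shot handler unbinds itself once its tag matches.
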(event `self.ReceiveBeginPlay`
  (bind _returnvalue (`|CreateWidget` "/Game/Widget/Event/WBP_Tutorial.WBP_Tutorial_C"))
  (`UserWidget.AddToViewport` _returnvalue 0))

(event `self.BP_OnOwningNarrtionUIComponentInitialized`
  (params (OwningPlayerComponent :type "NarrationalUIComponent Object Reference"))
  (bind _output_get (set `self.Owning Player Component` OwningPlayerComponent))
  (add `NarrationalUIComponent.NarrationEnded` _output_get (delegate `NarrationEnded_이벤트`)))

(event `NarrationEnded_이벤트`
  (params (Event_Tag :type "GameplayTag Structure (by ref)"))
  (if (== Event_Tag (struct :`TagName` "Call.00.Tutorial"))
    (remove `NarrationalUIComponent.NarrationEnded` (stale `self.BP_OnOwningNarrtionUIComponentInitialized` _output_get) (delegate `NarrationEnded_이벤트`))
    (`KismetSystemLibrary.Delay` 3.0)
    (`NarrationalUIComponent.TriggerNarration` (stale `self.BP_OnOwningNarrtionUIComponentInitialized` _output_get) "Sub.00.Room2")
    (add `NarrationalUIComponent.NarrationEnded` (stale `self.BP_OnOwningNarrtionUIComponentInitialized` _output_get) (delegate `NarrationEnded_이벤트_0`))))

(event `NarrationEnded_이벤트_0`
  (params (Event_Tag :type "GameplayTag Structure (by ref)"))
  (if (== Event_Tag (struct :`TagName` "Sub.00.Room2"))
    (remove `NarrationalUIComponent.NarrationEnded` (stale `self.BP_OnOwningNarrtionUIComponentInitialized` OwningPlayerComponent) (delegate `NarrationEnded_이벤트_0`))
    (`KismetSystemLibrary.Delay` 5.0)
    (`self.EndChapter` (struct :`TagName` "Chapter.00.Warehouse"))))

(fn `UserConstructionScript`)