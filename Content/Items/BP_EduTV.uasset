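; BP_EduTV is an interactable TV that plays the intro tutorial video once.
; On interact, if no narration is playing, it disables its interaction, records the watched event in the game instance and plays MS_Intro in a full-screen media widget.
; When the video ends, it removes the widget and triggers the first quest narration.
; BeginPlay keeps it disabled if the watched event already exists.
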(event `self.ReceiveBeginPlay`
  (bind _interactionhandler (`self.InteractionHandler`))
  (if (`NPGameInstance.HasEventOccurred` (`NPFunctionLibrary.GetNPGameInstance`) (struct :`TagName` "Event.Watched.TutorialVideo"))
    (set `InteractUIComponent.bInteractable` false _interactionhandler)
    (`InteractUIComponent.HideIcon` _interactionhandler)))

(event `InteractInterface.Interact`
  (params (Interactor :type "Actor Object Reference"))
  (bind _interactionhandler (`self.InteractionHandler`))
  (bind _media (`self.Media`))
  ; Interact Setting
  (bind _asnpplayer_character (cast `NPPlayerCharacter` Interactor))
  (bind _output_get (set `self.Narration Component` (`NPPlayerCharacter.NarrationComponent` _asnpplayer_character)))
  (if (`NarrationalUIComponent.IsNarrationPlaying` _output_get)
    _
    (elif (`InteractUIComponent.bInteractable` _interactionhandler)
      (set `InteractUIComponent.bInteractable` false _interactionhandler)
      (`InteractUIComponent.HideIcon` _interactionhandler)
      (`NPGameInstance.AddEvent` (`NPFunctionLibrary.GetNPGameInstance`) (struct :`TagName` "Event.Watched.TutorialVideo"))
      ; Play Media
      (bind _returnvalue (`|CreateWidget` "/Game/Widget/Event/WBP_MediaPlayer.WBP_MediaPlayer_C"))
      (`UserWidget.AddToViewport` _returnvalue 0)
      (`MediaPlayer.OpenSource` _media "/Game/Assets/Media/MS_Intro.MS_Intro")
      (add `MediaPlayer.OnEndReached` _media (delegate `OnEndReached_이벤트`)))))

(event `OnEndReached_이벤트`
  ; Play Media
  (`Widget.RemoveFromParent` (stale `InteractInterface.Interact` _returnvalue))
  (remove `MediaPlayer.OnEndReached` (`self.Media`) (delegate `OnEndReached_이벤트`))
  (`NarrationalUIComponent.TriggerNarration` (`self.Narration Component`) "Sub.00.Quest01"))

(fn `UserConstructionScript`)