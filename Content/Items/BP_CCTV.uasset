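; Interactable CCTV monitor that, once the tutorial video is watched, lets the player switch between security cameras through a button widget; otherwise narration rejects it.
; Button presses change the view target within CCTVList, with button 0 returning to the player.
; In the FindCart chapter exit is blocked and presses feed a DoOnce-gated camera puzzle, whose end event restores the player view, disables interaction and triggers radio narration.
; Interaction starts disabled in the Escape chapter.
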(event `self.ReceiveBeginPlay`
  (if (== (`NPGameInstance.GetCurrentChapter` (`NPFunctionLibrary.GetNPGameInstance`)) (struct :`TagName` "Chapter.00.Escape"))
    (bind _output_get (set `InteractUIComponent.bInteractable` false (`self.InteractionHandler`)))))

(event `InteractInterface.Interact`
  (params (Interactor :type "Actor Object Reference"))
  ; pre_setting
  (bind _asnpplayer_character (cast `NPPlayerCharacter` Interactor))
  (bind _output_get (set `self.Narration Component` (`NPPlayerCharacter.NarrationComponent` _asnpplayer_character)))
  (if (stale `self.ReceiveBeginPlay` _output_get)
    (if (`NPGameInstance.HasEventOccurred` (`NPFunctionLibrary.GetNPGameInstance`) (struct :`TagName` "Event.Watched.TutorialVideo"))
      (bind _asnpplayer_controller (cast `NPPlayerController` (`GameplayStatics.GetPlayerController` 0)))
      (bind _output_get_2 (set `self.As NPPlayer Controller` _asnpplayer_controller))
      (`PlayerController.SetViewTargetWithBlend` _output_get_2 (`|GetArrayItem` (`self.CCTV_List`)) 0.0 "VTBlend_Cubic" 0.0 false)
      (`NPPlayerController.SetUIInputMode` _asnpplayer_controller true)
      (`GameplayStatics.SetGamePaused` false)
      (`InteractUIComponent.HideIcon` (`self.InteractionHandler`))
      ; CCTV Logic
      (bind _returnvalue (`|CreateWidget` "/Game/Widget/Event/WBP_CCTV.WBP_CCTV_C"))
      (bind _output_get_3 (set `self.ButtonPannel` _returnvalue))
      (`UserWidget.AddToViewport` _returnvalue 0)
      (`UserWidget.AddToViewport` _output_get_3 0)
      (add `/Game/Widget/Event/WBP_CCTV.BT_CCTV` _output_get_3 (delegate `BT_CCTV_이벤트`))
      (if (== (`NPGameInstance.GetCurrentChapter` (`NPFunctionLibrary.GetNPGameInstance`)) (struct :`TagName` "Chapter.00.FindCart"))
        (add `NPCH0Component.OnCCTVEnded` (`self.CCTVComponent`) (delegate `OnCCTVEnded_이벤트`)))
      (else
        (`NarrationalUIComponent.TriggerNarration` _output_get "Sub.Reject.MonitorDoor")))))

(event `OnCCTVEnded_이벤트`
  (bind _cctvcomponent (`self.CCTVComponent`))
  (bind _buttonpannel (`self.ButtonPannel`))
  (bind _as_npplayer_controller (`self.As NPPlayer Controller`))
  ; CCTV Logic
  (remove `NPCH0Component.OnCCTVEnded` _cctvcomponent (delegate `OnCCTVEnded_이벤트`))
  (remove `/Game/Widget/Event/WBP_CCTV.BT_CCTV` _buttonpannel (delegate `BT_CCTV_이벤트`))
  (`KismetSystemLibrary.Delay` (`NPCH0Component.EventSec` _cctvcomponent))
  (`Widget.RemoveFromParent` _buttonpannel)
  (`NPPlayerController.SetUIInputMode` _as_npplayer_controller false)
  (set `InteractUIComponent.bInteractable` false (`self.InteractionHandler`))
  (`PlayerController.SetViewTargetWithBlend` _as_npplayer_controller (`GameplayStatics.GetPlayerPawn` 0) 0.0 "VTBlend_Cubic" 0.0 false)
  (`KismetSystemLibrary.Delay` (`NPCH0Component.GroupEventMin` _cctvcomponent))
  (`NarrationalUIComponent.TriggerNarration` (`self.Narration Component`) "Sub.00.Radio"))

(event `BT_CCTV_이벤트`
  (params (BTNum :type Integer))
  (bind _as_npplayer_controller (`self.As NPPlayer Controller`))
  (bind _buttonpannel (`self.ButtonPannel`))
  ; CCTV Logic
  (if (== (`NPGameInstance.GetCurrentChapter` (`NPFunctionLibrary.GetNPGameInstance`)) (struct :`TagName` "Chapter.00.FindCart"))
    (`/Engine/EditorBlueprintResources/StandardMacros.DoOnce` false :!label _label
      (:`Completed`
        (switch `int` BTNum
          (:`Default`
            (`PlayerController.SetViewTargetWithBlend` (`self.As NPPlayer Controller`) (`|GetArrayItem` (`self.CCTV_List`) BTNum) 0.0 "VTBlend_Linear" 0.0 false)
            (bind _returnvalue (`self.PuzzleCCTV` BTNum))
            (if _returnvalue
              (`KismetSystemLibrary.Delay` (`NPCH0Component.EventSec` (`self.CCTVComponent`)))
              (goto _label :!via `Reset`)
              (else
                (goto _label :!via `Reset`))))
          (:`0`
            (goto _label :!via `Reset`)))))
    (else
      (switch `int` BTNum
        (:`Default`
          (`PlayerController.SetViewTargetWithBlend` _as_npplayer_controller (`|GetArrayItem` (`self.CCTV_List`) BTNum) 0.0 "VTBlend_Linear" 0.0 false))
        (:`0`
          (remove `/Game/Widget/Event/WBP_CCTV.BT_CCTV` _buttonpannel (delegate `BT_CCTV_이벤트`))
          (`Widget.RemoveFromParent` _buttonpannel)
          (`NPPlayerController.SetUIInputMode` _as_npplayer_controller false)
          (set `InteractUIComponent.bInteractable` true (`self.InteractionHandler`))
          (`PlayerController.SetViewTargetWithBlend` _as_npplayer_controller (`GameplayStatics.GetPlayerPawn` 0) 0.0 "VTBlend_Cubic" 0.0 false))))))

(fn `UserConstructionScript`)