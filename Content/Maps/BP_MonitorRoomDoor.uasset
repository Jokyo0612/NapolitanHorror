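; Monitor room door that stays locked until the player has watched the tutorial video.
; On interaction it checks the game instance for that event, then either opens once and hides the interaction icon or triggers a rejection narration on the player.
; Ending actor overlap closes the door and resets the DoOnce so it can open again.
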(event `InteractInterface.Interact`
  (params (Interactor :type "Actor Object Reference"))
  (bind _asnpplayer_character (cast `NPPlayerCharacter` Interactor))
  (if (`NPGameInstance.HasEventOccurred` (`NPFunctionLibrary.GetNPGameInstance`) (struct :`TagName` "Event.Watched.TutorialVideo"))
    (`/Engine/EditorBlueprintResources/StandardMacros.DoOnce` false :!label _label
      (:`Completed`
        (`self.DoorOpen`)
        (`InteractUIComponent.HideIcon` (`self.InteractionHandler`))))
    (else
      (`NarrationalUIComponent.TriggerNarration` (`NPPlayerCharacter.NarrationComponent` _asnpplayer_character) "Sub.Reject.MonitorDoor"))))

(event `self.ReceiveActorEndOverlap`
  (params (OtherActor :type "Actor Object Reference"))
  (`self.DoorClose`)
  (goto _label :!via `Reset`))

(fn `UserConstructionScript`
  (`parent.UserConstructionScript`))