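; BP_LightShadow is a one-shot Stage0 scripted event where a spotlight changes intensity while a shadow slides across when the player overlaps it.
; A timeline drives light and shadow, with player move input locked shortly after it starts.
; On finish it restores input, triggers narration and the cart's interact message, then destroys itself.
; BeginPlay removes the actor if the game instance already records the event as watched.
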(event `self.ReceiveBeginPlay`
  (bind _asnpgame_instance (cast `NPGameInstance` (`GameplayStatics.GetGameInstance`)))
  (if (`NPGameInstance.HasEventOccurred` _asnpgame_instance (struct :`TagName` "Event.Watched.ShadowLight"))
    (`self.K2_DestroyActor`)))

(event `self.ReceiveActorBeginOverlap`
  (params (OtherActor :type "Actor Object Reference"))
  (bind _returnvalue (`GameplayStatics.GetPlayerController` 0))
  (bind _as_bp_npplayer_character (`self.As BP NPPlayer Character`))
  (bind _asbp_npplayer_character (cast `/Game/CustomPlayer/BP_NPPlayerCharacter` OtherActor))
  (set `self.As BP NPPlayer Character` _asbp_npplayer_character)
  (`/Engine/EditorBlueprintResources/StandardMacros.DoOnce` false
    (:`Completed`
      (`|ExecutionSequence`
        (:`then_0`
          ; Event Control
          (bind (_direction _light_tick _actor_y) (`Timeline|타임라인`)
            (:`Update`
              (`LightComponent.SetIntensity` (`self.SpotLight`) (* _light_tick 3000.0))
              (`SceneComponent.K2_SetRelativeLocation` (`self.Shadow`) (`KismetMathLibrary.MakeVector` (`KismetMathLibrary.Lerp` 200.0 -200.0 _actor_y) 0.0 -45.0) false false))
            (:`Finished`
              (`Controller.ResetIgnoreMoveInput` _returnvalue)
              (`KismetSystemLibrary.Delay` 1.5)
              (`NarrationalUIComponent.TriggerNarration` (`NPPlayerCharacter.NarrationComponent` _as_bp_npplayer_character) "Sub.00.ShadowLight")
              (`KismetSystemLibrary.Delay` 1.0)
              (message `InteractInterface.Interact` (`/Game/CustomPlayer/BP_NPPlayerCharacter.Cart_Cache` _as_bp_npplayer_character) _as_bp_npplayer_character)
              (`self.K2_DestroyActor`))))
        (:`then_1`
          (`KismetSystemLibrary.Delay` 1.5)
          (`Controller.SetIgnoreMoveInput` _returnvalue true))))))

(fn `UserConstructionScript`)