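; BP_DarkWall is a Stage0 actor that moves its ItemCollisionBox along a spline once StartEvent runs.
; A timeline maps its track to spline distance, and SplineSetter applies world location and a rotation taken from the spline's local-space direction.
; On the first game instance state change after starting, it unbinds, stops the timeline after a short delay, then snaps the box back to the spline start.
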(event `self.StartEvent`
  (add `NPGameInstance.OnGameStateChanged` (`NPFunctionLibrary.GetNPGameInstance`) (delegate `OnGameStateChanged_이벤트`))
  (bind (_direction `_새_트랙_0`) (`Timeline|타임라인` :!via `PlayFromStart` :!label _label)
    (:`Update`
      (bind _returnvalue (`KismetMathLibrary.Lerp` 0.0 (`SplineComponent.GetSplineLength` (`self.Spline`)) `_새_트랙_0`))
      (`self.SplineSetter` _returnvalue _returnvalue))))

(event `OnGameStateChanged_이벤트`
  (params (CurrentState :type "ENPGameState Enum" :default "WaitingToStart"))
  (remove `NPGameInstance.OnGameStateChanged` (`NPFunctionLibrary.GetNPGameInstance`) (delegate `OnGameStateChanged_이벤트`))
  (`|ExecutionSequence`
    (:`then_0`
      (`KismetSystemLibrary.Delay` 2.0)
      (goto _label :!via `Stop`))
    (:`then_1`
      (`KismetSystemLibrary.Delay` 2.01)
      (`self.SplineSetter` 0.0))))

(fn `SplineSetter`
  (params (Distance :type "Float (single-precision)") (Distance1 :type "Float (single-precision)"))
  (bind _spline (`self.Spline`))
  (`SceneComponent.K2_SetWorldLocationAndRotation` (`self.ItemCollisionBox`) (`SplineComponent.GetLocationAtDistanceAlongSpline` _spline Distance "World") (`KismetMathLibrary.Conv_VectorToRotator` (`SplineComponent.GetDirectionAtDistanceAlongSpline` _spline Distance1 "Local")) false false))

(fn `UserConstructionScript`)