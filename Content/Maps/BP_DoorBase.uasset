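; Base door actor that swings its Hinge open and shut with a timeline-driven rotation lerp.
; DoorOpen picks a positive or negative 90-degree yaw target from RelativePositionCaculation, whose player-side dot-product check appears unused in its graph.
; DoorClose reverses the timeline.
; Interact and ActorEndOverlap are empty, and the sample open/close logic with icon hiding is disconnected.
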(event `DoorOpen`
  (if (>= (`KismetMathLibrary.Dot_VectorVector` (`self.GetActorForwardVector`) (`KismetMathLibrary.Normal` (- (`self.K2_GetActorLocation` (`GameplayStatics.GetPlayerCharacter` 0)) (`self.K2_GetActorLocation`)))) 0.0)
    (set `self.B` (struct :`Yaw` 90.0))
    (bind (_direction `_새_트랙_0`) (`Timeline|Door_anime` :!via `PlayFromStart` :!label _label)
      (:`Update`
        (`SceneComponent.K2_SetRelativeRotation` (`self.Hinge`) (`KismetMathLibrary.RLerp` (struct) (`self.B`) `_새_트랙_0` true) false false)))
    (else
      (set `self.B` (struct :`Yaw` -90.0))
      (goto _label :!via `PlayFromStart`))))

(event `DoorClose`
  (goto _label :!via `Reverse`))

(event `InteractInterface.Interact`
  (params (Interactor :type "Actor Object Reference"))
  ; Sample Open Logic
)

(event `self.ReceiveActorEndOverlap`
  (params (OtherActor :type "Actor Object Reference"))
  ; Sample Open Logic
)

(fn `UserConstructionScript`)