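; Interactable bed that ends the current chapter when the player uses it.
; It is interactable from BeginPlay, and an Interactable function can set that flag again, though nothing here clears it.
; Interacting fades the camera out, waits, lifts the fade and plays the LS_Clock sequence.
; After another delay, it calls EndChapter on NPBaseGamemode with the Chapter.00.Warehouse tag.
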(event `self.ReceiveBeginPlay`
  (set `InteractUIComponent.bInteractable` true (`self.InteractionHandler`)))

(event `InteractInterface.Interact`
  (params (Interactor :type "Actor Object Reference"))
  (bind _returnvalue (`GameplayStatics.GetPlayerCameraManager` 0))
  (if (`InteractUIComponent.bInteractable` (`self.InteractionHandler`))
    (`PlayerCameraManager.StartCameraFade` :`self` _returnvalue :`ToAlpha` 1.0 :`Duration` 2.0 :`bHoldWhenFinished` true)
    (`KismetSystemLibrary.Delay` 4.0)
    (`PlayerCameraManager.StopCameraFade` _returnvalue)
    (bind (_outactor _returnvalue_2) (`LevelSequencePlayer.CreateLevelSequencePlayer` "/Game/Scenematic/LS_Clock.LS_Clock"))
    (`MovieSceneSequencePlayer.Play` _returnvalue_2)
    (`KismetSystemLibrary.Delay` 4.0)
    (bind _asnpbase_gamemode (cast `NPBaseGamemode` (`GameplayStatics.GetGameMode`)))
    (`NPBaseGamemode.EndChapter` _asnpbase_gamemode (struct :`TagName` "Chapter.00.Warehouse"))))

(fn `Interactable`
  (set `InteractUIComponent.bInteractable` true (`self.InteractionHandler`)))

(fn `UserConstructionScript`)